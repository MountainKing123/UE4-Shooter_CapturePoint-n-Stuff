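; Central capture point actor that a lone FirstPersonCharacter captures and holds by standing inside its Box.
; Overlap events track occupants in EnteredPlayers, starting capture for one player and stopping capture and hold when contested or empty.
; An authority-gated Timeline drives capture; on finish it flags occupants as holders, hard-codes team 1 and starts a looping Holding timer.
; Holding only prints debug ticket messages, without awarding any tickets.
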(event OnComponentBeginOverlap(Box)
  (params (OtherActor :type Actor%20Object%20Reference) (OtherComp :type Primitive%20Component%20Object%20Reference) (OtherBodyIndex :type Integer) (bFromSweep :type Boolean) (SweepResult :type Hit%20Result%20Structure%20%28by%20ref%29))
  (bind _enteredplayers (Variables|Default|GetEnteredPlayers))
  (bind _returnvalue (Utilities|Array|Length _enteredplayers))
  (bind _asfirst_person_character (Utilities|Casting|CastToFirstPersonCharacter OtherActor)
    (:then
      (Utilities|Array|AddUnique (Variables|Default|GetEnteredPlayers) _asfirst_person_character)
      (Development|PrintString "player entered" true true "(R=0.094116,G=1.000000,B=0.000000,A=1.000000)")
      (if (> _returnvalue 0)
        (if (> _returnvalue 1)
          (CallFunction|ServerEndCapture :!label _label)
          (CallFunction|ServerStopHolding)
          (elif (not (Variables|Default|GetisCapturing))
            (CallFunction|ServerStartCapture)))
        (else
          (goto _label))))
    (:CastFailed
      (Development|PrintString "YOU NO PLAYER!"))))

(event OnComponentEndOverlap(Box)
  (params (OtherActor :type Actor%20Object%20Reference) (OtherComp :type Primitive%20Component%20Object%20Reference) (OtherBodyIndex :type Integer))
  (bind _enteredplayers (Variables|Default|GetEnteredPlayers))
  (bind _enteredplayers_2 (Variables|Default|GetEnteredPlayers))
  (bind _returnvalue (Utilities|Array|Length _enteredplayers_2))
  (bind _asfirst_person_character (Utilities|Casting|CastToFirstPersonCharacter OtherActor)
    (:then
      (for (_array_element _array_index) _enteredplayers
        (if (== _array_element _asfirst_person_character)
          (Variables|/Game/Blueprints/FirstPersonBP/Blueprints/FirstPersonCharacter.FirstPersonCharacter_C|SetisHoldingCentralPoint _array_element false)
          (Utilities|Array|RemoveIndex _enteredplayers _array_index)
          (Development|PrintString "player left point" true true "(R=1.000000,G=0.062643,B=0.000000,A=1.000000)")
          (else
            (Development|PrintString "LOL"))))
      (if (> _returnvalue 0)
        (if (> _returnvalue 1)
          (CallFunction|ServerEndCapture :!label _label)
          (CallFunction|ServerStopHolding)
          (else
            (CallFunction|ServerStartCapture)))
        (else
          (goto _label))))
    (:CastFailed
      (Development|PrintString "LOL"))))

(event Custom|ServerStartCapture
  (Networking|SwitchHasAuthority
    (:Authority
      (Variables|Default|SetisCapturing true)
      (bind _holdtime (Timeline|Timeline_0 PlayFromStart)
        (:Update
          (bind _output_get (Variables|Default|SetCurrentHoldTime%20 _holdtime))
          (Development|PrintString (Utilities|String|ToString(Float) _output_get)))
        (:Finished
          (CallFunction|ServerIsHoldingPoint)
          (Variables|Default|SetisHold true))))))

(event Custom|ServerIsHoldingPoint
  (Networking|SwitchHasAuthority
    (:Authority
      (bind _returnvalue (Utilities|Time|SetTimerbyFunctionName 0 "Holding" 3.0 true))
      (for _array_element (Variables|Default|GetEnteredPlayers)
        (Variables|/Game/Blueprints/FirstPersonBP/Blueprints/FirstPersonCharacter.FirstPersonCharacter_C|SetisHoldingCentralPoint _array_element true)
        (Variables|Default|SetHoldingTeamInt 1)))))

(event Custom|ServerEndCapture
  (Variables|Default|SetisCapturing false)
  (bind _holdtime (Timeline|Timeline_0 Stop)
    (:Update
      (bind _output_get (Variables|Default|SetCurrentHoldTime%20 _holdtime))
      (Development|PrintString (Utilities|String|ToString(Float) _output_get)))
    (:Finished
      (CallFunction|ServerIsHoldingPoint)
      (Variables|Default|SetisHold true))))

(event Custom|ServerStopHolding
  (Class|KismetSystemLibrary|ClearTimerHandle (stale Custom|ServerIsHoldingPoint _returnvalue))
  (Variables|Default|SetisHold false)
  (Variables|Default|SetisCapturing false)
  (Variables|Default|SetHoldingTeamInt 0))

(event EventBeginPlay)

(event EventActorBeginOverlap
  (params (OtherActor :type Actor%20Object%20Reference)))

(event EventTick
  (params (DeltaSeconds :type Float%20%28single-precision%29)))

(fn ConstructionScript)

(fn Holding
  (for _array_element (Variables|Default|GetEnteredPlayers)
    (Development|PrintString (Utilities|String|Append (Utilities|GetDisplayName _array_element) "is capturing" "+" (Utilities|String|ToString(Integer) (Variables|Default|GetCaptureTickets))))))