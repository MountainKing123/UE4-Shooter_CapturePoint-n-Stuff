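; Multiplayer player controller that handles HUD setup, respawning after team selection and chat input.
; After login it waits briefly, then SetupIngameUI creates the W_MPHUD widget and adds it to the viewport for local controllers only.
; PostTeamSelection asks GM_MPGameMode to respawn the player, while the Chat action tells FirstPersonHUD to begin message typing.
; Some widget-removal, input-mode and respawn nodes are left unconnected.
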(event Custom|ClientPostLogin
  (Utilities|FlowControl|Delay 0.5)
  (CallFunction|SetupIngameUI)
  (bind _asgm_mpgame_mode (Utilities|Casting|CastToGM_MPGameMode (Game|GetGameMode))))

(event Custom|PostTeamSelection
  (bind _asgm_mpgame_mode (Utilities|Casting|CastToGM_MPGameMode (Game|GetGameMode)))
  (Default|RespawnPlayerEvent _asgm_mpgame_mode self))

(event EventEndPlay
  (params (EndPlayReason :type EEndPlayReason%20Enum :default "Destroyed"))
  ;[1 1 1] gives error
)

(event Input|ActionEvents|InputActionChat
  (params (Key :type Key%20Structure :default "AnyKey"))
  (:Pressed
    (bind _asfirst_person_hud (Utilities|Casting|CastToFirstPersonHUD (HUD|GetHUD)))
    (Default|CallOnPlayerBeginTypeChatMsg _asfirst_person_hud)))

(fn ConstructionScript)

(fn SetupIngameUI
  (if (Pawn|IsLocalPlayerController)
    (bind _returnvalue (UserInterface|CreateWidget "/Game/Blueprints/Multiplayer/Widgets/W_MPHUD.W_MPHUD_C" self))
    (bind _output_get (Variables|Default|SetHUDWidget _returnvalue))
    (UserInterface|Viewport|AddtoViewport _output_get 0)))